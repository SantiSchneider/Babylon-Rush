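; Bomb enemy that damages nearby pawns by exploding, with a short forward sphere-trace melee attack.
; A random BeginPlay timer triggers a radial explosion and destroys the actor.
; Death ragdolls the mesh, then after a short delay deals damage in a wider radius without destroying the actor.
; BPCDamageSystem handles health, damage and the death binding; Heal is a stub, and attacks draw debug shapes.
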(event Custom|Death%20Event
  (bind _mesh (Variables|Character|GetMesh))
  (Pawn|Components|CharacterMovement|SetMovementMode (Variables|Character|GetCharacterMovement) "MOVE_None" 0)
  (Physics|SetSimulatePhysics _mesh true)
  (Collision|SetCollisionEnabled _mesh "QueryAndPhysics")
  (Utilities|FlowControl|Delay 1.0)
  (Rendering|Debug|DrawDebugSphere (Transformation|GetActorLocation) 3e+02 12 "(R=1.000000,G=0.129164,B=0.228875,A=1.000000)" 4.0 3.0)
  (bind _outactors (Collision|SphereOverlapActors (Transformation|GetActorLocation) 3e+02 (Utilities|Array|MakeArray "ObjectTypeQuery3") 0))
  (Class|BPIDamagable|TakeDamage(Message) _outactors (Utilities|Struct|MakeS_Damagable 7e+01 "NewEnumerator3")))

(event Custom|Damage%20Response
  (params (Damage%20Response :type Byte :default 0)))

(event Custom|Attack
  (bind _returnvalue (Transformation|GetActorLocation))
  (bind (_outhit _returnvalue_2) (Collision|SphereTraceForObjects _returnvalue (+ _returnvalue (* (Transformation|GetActorForwardVector) 1e+02)) 2e+01 (Utilities|Array|MakeArray "ObjectTypeQuery3") false 0 "ForDuration" true "(R=1.000000,G=0.000000,B=0.000000,A=1.000000)" "(R=0.000000,G=1.000000,B=0.000000,A=1.000000)" 2.0))
  (if _returnvalue_2
    (Class|BPIDamagable|TakeDamage(Message) (.HitActor (Collision|BreakHitResult _outhit)) (Utilities|Struct|MakeS_Damagable 15.0 "NewEnumerator1"))))

(event Custom|AoE%20Explosion
  (Rendering|Debug|DrawDebugSphere (Transformation|GetActorLocation) 2e+02 12 "(R=1.000000,G=0.081855,B=0.131617,A=1.000000)" 4.0 2.0)
  (bind _outactors (Collision|SphereOverlapActors (Transformation|GetActorLocation) 2e+02 (Utilities|Array|MakeArray "ObjectTypeQuery3") 0))
  (Class|BPIDamagable|TakeDamage(Message) _outactors (Utilities|Struct|MakeS_Damagable 7e+01 "NewEnumerator3"))
  (Actor|DestroyActor))

(event EventBeginPlay
  (Utilities|Time|SetTimerbyEvent (delegate Custom|AoE%20Explosion) (Math|Random|RandomFloatinRange 5e+01 1e+02)))

(fn ConstructionScript
  (EventDispatchers|BindEventtoOnDeath (Variables|Default|GetBPC_DamageSystem) (EventDispatchers|CreateEvent :!event Custom|Death%20Event)))

(fn GetCurrentHealth
  (return (Variables|/Game/DamageSystem/BPC_DamageSystem.BPC_DamageSystem_C|GetHealth (Variables|Default|GetBPC_DamageSystem))))

(fn GetMaxHealth
  (return (Variables|/Game/DamageSystem/BPC_DamageSystem.BPC_DamageSystem_C|GetMaxHealth (Variables|Default|GetBPC_DamageSystem))))

(fn Heal
  (params (Amount :type Float%20%28double-precision%29))
  (return 0.0))

(fn TakeDamage
  (params (DamageInfo :type S%20Damagable%20Structure))
  (bind _wasdamaged (Default|TakeDamage (Variables|Default|GetBPC_DamageSystem) DamageInfo))
  (return _wasdamaged))