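; Ranged enemy character that fires projectiles and can be damaged and killed.
; BPCDamageSystem handles health and damage behind the damageable functions, which feed a widget health bar; Heal is a stub.
; Attack spawns BP_Projectile_Enemy at a scene component and binds its impact event to deal fixed damage to the hit actor.
; The component's death event, bound in the construction script, stops movement, ragdolls the mesh and destroys the actor after a short delay.
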(event Custom|Death%20Event
  (bind _mesh (Variables|Character|GetMesh))
  (Pawn|Components|CharacterMovement|SetMovementMode (Variables|Character|GetCharacterMovement) "MOVE_None" 0)
  (Physics|SetSimulatePhysics _mesh true)
  (Collision|SetCollisionEnabled _mesh "QueryAndPhysics")
  (Utilities|FlowControl|Delay 1.0)
  (Actor|DestroyActor))

(event Custom|Damage%20Response
  (params (Damage%20Response :type Byte :default 0)))

(event Custom|Attack
  (bind _returnvalue (Game|SpawnActorfromClass "/Game/Projectiles/BP_Projectile_Enemy.BP_Projectile_Enemy_C" (Transformation|GetWorldTransform (Variables|Default|GetScene)) "Undefined" "MultiplyWithRoot" self 3e+02 0.0 0))
  (EventDispatchers|BindEventtoOnImpact _returnvalue (delegate Custom|HitPlayer))
  (Collision|IgnoreActorwhenMoving (Variables|Collision|GetCapsuleComponent) _returnvalue true))

(event Custom|HitPlayer
  (params (Actor :type Actor%20Object%20Reference) (Hit :type Hit%20Result%20Structure))
  (Class|BPIDamagable|TakeDamage(Message) Actor (Utilities|Struct|MakeS_Damagable 5e+01 "NewEnumerator2")))

(event EventBeginPlay
  (bind _returnvalue (UserInterface|CreateWidget "/Game/UI/W_HealthBar.W_HealthBar_C" 0 self))
  (UserInterface|SetWidget (Variables|Default|GetWidget) _returnvalue))

(fn ConstructionScript
  (EventDispatchers|BindEventtoOnDeath (Variables|Default|GetBPC_DamageSystem) (EventDispatchers|CreateEvent :!event Custom|Death%20Event)))

(fn GetCurrentHealth
  (return (Variables|/Game/DamageSystem/BPC_DamageSystem.BPC_DamageSystem_C|GetHealth (Variables|Default|GetBPC_DamageSystem))))

(fn GetMaxHealth
  (return (Variables|/Game/DamageSystem/BPC_DamageSystem.BPC_DamageSystem_C|GetMaxHealth (Variables|Default|GetBPC_DamageSystem))))

(fn Heal
  (params (Amount :type Float%20%28double-precision%29))
  (return 0.0))

(fn TakeDamage
  (params (DamageInfo :type S%20Damagable%20Structure))
  (bind _wasdamaged (Default|TakeDamage (Variables|Default|GetBPC_DamageSystem) DamageInfo))
  (return _wasdamaged))