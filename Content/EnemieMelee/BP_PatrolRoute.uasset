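; Patrol route actor, filed under melee enemy assets, that supplies world-space waypoints from its PatrolRoute spline.
; IncrementPR steps the Point index by Direction, and GetSplineWorldPosition returns that point's location.
; Direction flips for back-and-forth travel at index zero and at an upper bound.
; That bound subtracts -1 from the point count, so it lands at count plus one, beyond the last valid index.
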(event Custom|IncrementPR
  (bind _output_get (Variables|Default|SetPoint (+ (Variables|Default|GetPoint) (Variables|Default|GetDirection))))
  (if (== _output_get (- (Spline|GetNumberOfSplinePoints (Variables|Default|GetPatrol%20Route)) -1))
    (Variables|Default|SetDirection -1)
    (elif (== (Variables|Default|GetPoint) 0)
      (Variables|Default|SetDirection 1))))

(fn ConstructionScript)

(fn GetSplineWorldPosition
  (return (Spline|GetLocationatSplinePoint (Variables|Default|GetPatrol%20Route) (Variables|Default|GetPoint) "World")))