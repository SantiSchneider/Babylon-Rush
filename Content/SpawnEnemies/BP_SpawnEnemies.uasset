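; Wave spawner that runs three enemy waves, announces each through the W_EnemyCount widget, then shows the win screen.
; A looping timer switches on EnemyWave, spawning melee, ranged or bomb enemies by random rolls at three scene points until that wave's cumulative spawn cap.
; Bound death events count kills and decrement EnemiesRound; a wave advances when the cap is reached and that counter equals zero.
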(event Custom|wave1
  (bind _returnvalue (Math|Random|RandomIntegerinRange 0 100))
  (bind _returnvalue_2 (Math|Random|RandomIntegerinRange 0 100))
  (bind _returnvalue_3 (Math|Random|RandomIntegerinRange 0 100))
  (bind _wave_inf (Variables|Default|GetWave%20Inf))
  (bind _wave_inf_2 (Variables|Default|GetWave%20Inf))
  (switch int (Variables|Default|GetEnemyWave)
    (:0
      (if (< (Variables|Default|GetEnemyCount) 10)
        (switch int (Math|Random|RandomIntegerinRange 0 2)
          (:0
            (Variables|Default|SetSceneLocation (Transformation|GetWorldLocation (Variables|Default|GetScene))))
          (:1
            (Variables|Default|SetSceneLocation (Transformation|GetWorldLocation (Variables|Default|GetScene1))))
          (:2
            (Variables|Default|SetSceneLocation (Transformation|GetWorldLocation (Variables|Default|GetScene2)))))
        (if (< _returnvalue_2 50)
          (bind _returnvalue_4 (Game|SpawnActorfromClass "/Game/DamageSystem/Enemy/BP_test.BP_test_C" (Math|Conversions|ToTransform(Vector) (Variables|Default|GetSceneLocation)) "Undefined" "MultiplyWithRoot" 0 0 0))
          (EventDispatchers|BindEventtoEnemieMeleeDie _returnvalue_4 (delegate Custom|CustomEvent_7))
          (Variables|Default|SetEnemyCount (+ 1 (Variables|Default|GetEnemyCount)))
          (elif (and (>= _returnvalue_2 50) (<= _returnvalue_2 75))
            (bind _returnvalue_5 (Game|SpawnActorfromClass "/Game/Enemies/BP_Enemy_Range.BP_Enemy_Range_C" (Math|Conversions|ToTransform(Vector) (Variables|Default|GetSceneLocation)) "Undefined" "MultiplyWithRoot" 0 0 0))
            (EventDispatchers|BindEventtoEnemyDie _returnvalue_5 (delegate Custom|CustomEvent_8))
            (Variables|Default|SetEnemyCount (+ 1 (Variables|Default|GetEnemyCount)))
            (elif (> _returnvalue_2 75)
              (bind _returnvalue_6 (Game|SpawnActorfromClass "/Game/Enemies/BP_EnemyBomb.BP_EnemyBomb_C" (Math|Conversions|ToTransform(Vector) (Variables|Default|GetSceneLocation)) "Undefined" "MultiplyWithRoot" 0 0 0))
              (EventDispatchers|BindEventtoEnemyBombDie _returnvalue_6 (delegate Custom|CustomEvent_9))
              (Variables|Default|SetEnemyCount (+ 1 (Variables|Default|GetEnemyCount))))))
        (elif (== 0 (Variables|Default|GetEnemiesRound))
          (Variables|Default|SetEnemyWave (+ (Variables|Default|GetEnemyWave) 1)))))
    (:1
      (if (Variables|Default|GetWave2Anounc)
        (Variables|Default|SetWave2Anounc false)
        (Variables|Default|SetEnemiesRound 3)
        (Variables|Default|SetEnemyKills 0)
        (Default|UpdateWaveNumber _wave_inf_2 2)
        (Default|ShowWaveText _wave_inf_2)
        (Utilities|FlowControl|Delay 5.0)
        (Default|HideWaveText _wave_inf_2)
        (Utilities|FlowControl|Delay 5.0))
      (if (< (Variables|Default|GetEnemyCount) 30)
        (switch int (Math|Random|RandomIntegerinRange 0 2)
          (:0
            (Variables|Default|SetSceneLocation (Transformation|GetWorldLocation (Variables|Default|GetScene))))
          (:1
            (Variables|Default|SetSceneLocation (Transformation|GetWorldLocation (Variables|Default|GetScene1))))
          (:2
            (Variables|Default|SetSceneLocation (Transformation|GetWorldLocation (Variables|Default|GetScene2)))))
        (if (< _returnvalue_3 50)
          (bind _returnvalue_7 (Game|SpawnActorfromClass "/Game/DamageSystem/Enemy/BP_test.BP_test_C" (Math|Conversions|ToTransform(Vector) (Variables|Default|GetSceneLocation)) "Undefined" "MultiplyWithRoot" 0 0 0))
          (EventDispatchers|BindEventtoEnemieMeleeDie _returnvalue_7 (delegate Custom|CustomEvent_10))
          (Variables|Default|SetEnemyCount (+ 1 (Variables|Default|GetEnemyCount)))
          (elif (and (>= _returnvalue_3 50) (<= _returnvalue_3 75))
            (bind _returnvalue_8 (Game|SpawnActorfromClass "/Game/Enemies/BP_Enemy_Range.BP_Enemy_Range_C" (Math|Conversions|ToTransform(Vector) (Variables|Default|GetSceneLocation)) "Undefined" "MultiplyWithRoot" 0 0 0))
            (EventDispatchers|BindEventtoEnemyDie _returnvalue_8 (delegate Custom|CustomEvent_11))
            (Variables|Default|SetEnemyCount (+ 1 (Variables|Default|GetEnemyCount)))
            (elif (> _returnvalue_3 75)
              (bind _returnvalue_9 (Game|SpawnActorfromClass "/Game/Enemies/BP_EnemyBomb.BP_EnemyBomb_C" (Math|Conversions|ToTransform(Vector) (Variables|Default|GetSceneLocation)) "Undefined" "MultiplyWithRoot" 0 0 0))
              (EventDispatchers|BindEventtoEnemyBombDie _returnvalue_9 (delegate Custom|CustomEvent_12))
              (Variables|Default|SetEnemyCount (+ 1 (Variables|Default|GetEnemyCount))))))
        (elif (== 0 (Variables|Default|GetEnemiesRound))
          (Variables|Default|SetEnemyWave (+ (Variables|Default|GetEnemyWave) 1)))))
    (:2
      (if (Variables|Default|GetWave3Anounc)
        (Variables|Default|SetWave3Anounc false)
        (Variables|Default|SetEnemiesRound 3)
        (Variables|Default|SetEnemyKills 0)
        (Default|UpdateWaveNumber _wave_inf 3)
        (Default|ShowWaveText _wave_inf)
        (Utilities|FlowControl|Delay 5.0)
        (Default|HideWaveText _wave_inf)
        (Utilities|FlowControl|Delay 5.0))
      (if (< (Variables|Default|GetEnemyCount) 60)
        (switch int (Math|Random|RandomIntegerinRange 0 2)
          (:0
            (Variables|Default|SetSceneLocation (Transformation|GetWorldLocation (Variables|Default|GetScene))))
          (:1
            (Variables|Default|SetSceneLocation (Transformation|GetWorldLocation (Variables|Default|GetScene1))))
          (:2
            (Variables|Default|SetSceneLocation (Transformation|GetWorldLocation (Variables|Default|GetScene2)))))
        (if (< _returnvalue 50)
          (bind _returnvalue_10 (Game|SpawnActorfromClass "/Game/DamageSystem/Enemy/BP_test.BP_test_C" (Math|Conversions|ToTransform(Vector) (Variables|Default|GetSceneLocation)) "Undefined" "MultiplyWithRoot" 0 0 0))
          (EventDispatchers|BindEventtoEnemieMeleeDie _returnvalue_10 (delegate Custom|CustomEvent))
          (Variables|Default|SetEnemyCount (+ 1 (Variables|Default|GetEnemyCount)))
          (elif (and (>= _returnvalue 50) (<= _returnvalue 75))
            (bind _returnvalue_11 (Game|SpawnActorfromClass "/Game/Enemies/BP_Enemy_Range.BP_Enemy_Range_C" (Math|Conversions|ToTransform(Vector) (Variables|Default|GetSceneLocation)) "Undefined" "MultiplyWithRoot" 0 0 0))
            (EventDispatchers|BindEventtoEnemyDie _returnvalue_11 (delegate Custom|CustomEvent_1))
            (Variables|Default|SetEnemyCount (+ 1 (Variables|Default|GetEnemyCount)))
            (elif (> _returnvalue 75)
              (bind _returnvalue_12 (Game|SpawnActorfromClass "/Game/Enemies/BP_EnemyBomb.BP_EnemyBomb_C" (Math|Conversions|ToTransform(Vector) (Variables|Default|GetSceneLocation)) "Undefined" "MultiplyWithRoot" 0 0 0))
              (EventDispatchers|BindEventtoEnemyBombDie _returnvalue_12 (delegate Custom|CustomEvent_2))
              (Variables|Default|SetEnemyCount (+ 1 (Variables|Default|GetEnemyCount))))))
        (elif (== 0 (Variables|Default|GetEnemiesRound))
          (Variables|Default|SetEnemyWave (+ (Variables|Default|GetEnemyWave) 1)))))
    (:3
      (bind _returnvalue_13 (UserInterface|CreateWidget "/Game/UI/W_WinGame.W_WinGame_C"))
      (UserInterface|Viewport|AddtoViewport _returnvalue_13 0)
      (Variables|Default|SetEnd%20game true))))

(event Custom|CustomEvent_7
  (Variables|Default|SetEnemyKills (+ 1 (Variables|Default|GetEnemyKills)))
  (Variables|Default|SetEnemiesRound (- (Variables|Default|GetEnemiesRound) 1)))

(event Custom|CustomEvent
  (Variables|Default|SetEnemyKills (+ 1 (Variables|Default|GetEnemyKills)))
  (Variables|Default|SetEnemiesRound (- (Variables|Default|GetEnemiesRound) 1)))

(event Custom|CustomEvent_1
  (Variables|Default|SetEnemyKills (+ 1 (Variables|Default|GetEnemyKills)))
  (Variables|Default|SetEnemiesRound (- (Variables|Default|GetEnemiesRound) 1)))

(event Custom|CustomEvent_2
  (Variables|Default|SetEnemyKills (+ 1 (Variables|Default|GetEnemyKills)))
  (Variables|Default|SetEnemiesRound (- (Variables|Default|GetEnemiesRound) 1)))

(event Custom|CustomEvent_8
  (Variables|Default|SetEnemyKills (+ 1 (Variables|Default|GetEnemyKills)))
  (Variables|Default|SetEnemiesRound (- (Variables|Default|GetEnemiesRound) 1)))

(event Custom|CustomEvent_9
  (Variables|Default|SetEnemyKills (+ 1 (Variables|Default|GetEnemyKills)))
  (Variables|Default|SetEnemiesRound (- (Variables|Default|GetEnemiesRound) 1)))

(event Custom|CustomEvent_10
  (Variables|Default|SetEnemyKills (+ 1 (Variables|Default|GetEnemyKills)))
  (Variables|Default|SetEnemiesRound (- (Variables|Default|GetEnemiesRound) 1)))

(event Custom|CustomEvent_11
  (Variables|Default|SetEnemyKills (+ 1 (Variables|Default|GetEnemyKills)))
  (Variables|Default|SetEnemiesRound (- (Variables|Default|GetEnemiesRound) 1)))

(event Custom|CustomEvent_12
  (Variables|Default|SetEnemyKills (+ 1 (Variables|Default|GetEnemyKills)))
  (Variables|Default|SetEnemiesRound (- (Variables|Default|GetEnemiesRound) 1)))

(event EventBeginPlay
  (bind _returnvalue (UserInterface|CreateWidget "/Game/UI/W_EnemyCount.W_EnemyCount_C" (Game|GetPlayerController 0)))
  (bind _output_get (Variables|Default|SetWave%20Inf _returnvalue))
  (UserInterface|Viewport|AddtoViewport _output_get 0)
  (Default|UpdateWaveNumber (Variables|Default|GetWave%20Inf) 1)
  (Default|ShowWaveText (Variables|Default|GetWave%20Inf))
  (Variables|Default|SetEnemiesRound 3)
  (Utilities|FlowControl|Delay 5.0)
  (Default|HideWaveText (Variables|Default|GetWave%20Inf))
  (Utilities|FlowControl|Delay 1.0)
  (Utilities|Time|SetTimerbyEvent (delegate Custom|wave1) 2.0 true))

(fn ConstructionScript)